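; Speed-up pickup that temporarily accelerates the game and gives the player an additional boost.
; BeginPlay sets a negative-Y Speed vector, while ApplyEffect plays a coin sound and copies Value into DelayUntilNormalSpeed.
; While that is non-zero, Tick, after calling its parent, doubles both global and player custom time dilation, then restores both and clears it after a Delay, which runs in dilated time.
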(event `self.ReceiveBeginPlay`
  (set `self.Speed` (0.0 -2.0 0.0)))

(event `self.ReceiveTick`
  (params (DeltaSeconds :type "Float (single-precision)"))
  (`parent.ReceiveTick` DeltaSeconds)
  (if (!= (`self.DelayUntilNormalSpeed`) 0)
    (`GameplayStatics.SetGlobalTimeDilation` 2.0)
    (set `Actor.CustomTimeDilation` 2.0 (`GameplayStatics.GetPlayerCharacter` 0))
    (`KismetSystemLibrary.Delay` (`KismetMathLibrary.Conv_IntToDouble` (`self.DelayUntilNormalSpeed`)))
    (set `Actor.CustomTimeDilation` 1.0 (`GameplayStatics.GetPlayerCharacter` 0))
    (`GameplayStatics.SetGlobalTimeDilation` 1.0)
    (set `self.DelayUntilNormalSpeed` 0)))

(fn `ApplyEffect`
  (`GameplayStatics.PlaySound2D` "/Game/Sounds/coin.coin" 1.0 1.0 0.0 null null)
  (set `self.DelayUntilNormalSpeed` (`self.Value`)))

(fn `UserConstructionScript`)