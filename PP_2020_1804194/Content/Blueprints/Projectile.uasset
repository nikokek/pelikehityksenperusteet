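; Base-style moving projectile, also called a collectible, that the player character can hit, with an empty ApplyEffect hook.
; Each tick it moves by Speed scaled by global time dilation, without delta time or sweep.
; Overlaps are identified by object name: the player triggers ApplyEffect, and both player and respawn trigger recycle the actor.
; Recycling restores initial X/Y, randomizes height and applies a random uniform scale.
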(event `self.ReceiveTick`
  (params (DeltaSeconds :type "Float (single-precision)"))
  ;[1 1 1] Move collectible
  (`self.K2_AddActorWorldOffset` (* (`self.Speed`) (`GameplayStatics.GetGlobalTimeDilation`))))

(event `self.ReceiveActorBeginOverlap`
  (params (OtherActor :type "Actor Object Reference"))
  (bind _returnvalue (`KismetSystemLibrary.GetObjectName` OtherActor))
  ;[1 1 1] check if collectable hit boy
  (bind _hitresult (`self.Check Boy Hit` _returnvalue))
  (if _hitresult
    (`self.ApplyEffect`)
    ;[1 1 1] Reset position
    (`self.ResetPosition` :!label _label)
    (`self.ResetScale`)
    (else
      ;[1 1 1] if not boy, check if hit respawntrigger
      (bind _hitresult_2 (`self.CheckRespawnHit` _returnvalue))
      (if _hitresult_2
        (goto _label)))))

(fn `ApplyEffect`)

(fn `Check Boy Hit`
  (params (OtherObjectName :type String))
  (returns (HitResult :type Boolean))
  (return (`KismetStringLibrary.EqualEqual_StrStr` OtherObjectName (`KismetSystemLibrary.GetObjectName` (`GameplayStatics.GetPlayerCharacter` 0)))))

(fn `CheckRespawnHit`
  (params (OtherObjectName :type String))
  (returns (HitResult :type Boolean))
  (return (`KismetStringLibrary.EqualEqual_StrStr` OtherObjectName (`self.RespawntriggerName`))))

(fn `ResetPosition`
  (`self.K2_SetActorLocation` (`KismetMathLibrary.MakeVector` (.x (`self.InitialPosition`)) (.y (`self.InitialPosition`)) (`KismetMathLibrary.RandomFloatInRange` 100.0 400.0))))

(fn `ResetScale`
  (bind _output_get (set `self.Scale` (`KismetMathLibrary.RandomFloatInRange` 2.0 5.0)))
  (bind _returnvalue (/ _output_get 7.0))
  (`self.SetActorScale3D` (`KismetMathLibrary.MakeVector` _returnvalue _returnvalue _returnvalue)))

(fn `UserConstructionScript`)